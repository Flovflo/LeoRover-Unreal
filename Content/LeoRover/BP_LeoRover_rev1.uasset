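; Leo Rover Blueprint that drives a four-wheeled rover with skid steering through physics constraint angular motors.
; The construction script sets per-side drive strengths, and each Tick applies the summed forward and turn velocities as wheel targets.
; Two custom events derive those velocities from the sign of persistent linear and angular values, waking the wheel bodies when nonzero.
; Spring arm camera look code is present but disconnected.
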(event Custom|CustomEvent
  (params (DeltaSeconds :type Float%20%28single-precision%29))
  (bind _linearvelocity (Variables|Default|GetLinearVelocity))
  (bind _persistentlinearvelocity (Variables|Default|GetPersistentLinearVelocity))
  (bind _returnvalue (* -1.0 _linearvelocity))
  ;[1 1 1] Setup Forward Torque
  (if (Math|Float|NearlyEqual(Float) _persistentlinearvelocity 0.0 1e-06)
    (Variables|Default|SetLeftVelocity 0.0)
    (Variables|Default|SetRightVelocity 0.0)
    (else
      (if (> _persistentlinearvelocity 0.0)
        (Variables|Default|SetLeftVelocity _returnvalue)
        (Variables|Default|SetRightVelocity _returnvalue)
        (else
          (Variables|Default|SetLeftVelocity _linearvelocity)
          (Variables|Default|SetRightVelocity _linearvelocity)))
      (CallFunction|WakeRigidBody))))

(event Custom|CustomEvent_1
  (params (DeltaSeconds :type Float%20%28single-precision%29))
  (bind _angularvelocity (Variables|Default|GetAngularVelocity))
  (bind _persistentangularvelocity (Variables|Default|GetPersistentAngularVelocity))
  (bind _returnvalue (* -1.0 _angularvelocity))
  ;[1 1 1] Setup Steering Torque
  (if (Math|Float|NearlyEqual(Float) _persistentangularvelocity 0.0 1e-06)
    (Variables|Default|SetLeftTurnVelocity 0.0)
    (Variables|Default|SetRightTurnVelocity 0.0)
    (else
      (if (> _persistentangularvelocity 0.0)
        (Variables|Default|SetLeftTurnVelocity _returnvalue)
        (Variables|Default|SetRightTurnVelocity _angularvelocity)
        (else
          (Variables|Default|SetLeftTurnVelocity _angularvelocity)
          (Variables|Default|SetRightTurnVelocity _returnvalue)))
      (CallFunction|WakeRigidBody))))

(event EventBeginPlay
  ;[1 1 1] Configures on BeginPlay
)

(event EventTick
  (params (DeltaSeconds :type Float%20%28single-precision%29))
  (CallFunction|SetVelocity))

(event Input|AxisEvents|InputAxisLookUp
  (params (AxisValue :type Float%20%28single-precision%29))
  ;[1 1 1] Camera Control
)

(event Input|AxisEvents|InputAxisLookRight
  (params (AxisValue :type Float%20%28single-precision%29))
  ;[1 1 1] Camera Control
)

(fn ConstructionScript
  (CallFunction|SetAngularDriveParam))

(fn SetAngularDriveParam
  (bind _leftvelocitystrength (Variables|Default|GetLeftVelocityStrength))
  (bind _rightvelocitystrength (Variables|Default|GetRightVelocityStrength))
  (Class|PhysicsConstraintComponent|SetAngularDriveParams (Variables|Default|GetPC_WheelFL) 0.0 _leftvelocitystrength 0.0)
  (Class|PhysicsConstraintComponent|SetAngularDriveParams (Variables|Default|GetPC_WheelRL) 0.0 _leftvelocitystrength 0.0)
  (Class|PhysicsConstraintComponent|SetAngularDriveParams (Variables|Default|GetPC_WheelFR) 0.0 _rightvelocitystrength 0.0)
  (Class|PhysicsConstraintComponent|SetAngularDriveParams (Variables|Default|GetPC_WheelRR) 0.0 _rightvelocitystrength 0.0))

(fn SetVelocity
  (bind _leftturnvelocity (Variables|Default|GetLeftTurnVelocity))
  (bind _leftvelocity (Variables|Default|GetLeftVelocity))
  (bind _rightvelocity (Variables|Default|GetRightVelocity))
  (bind _rightturnvelocity (Variables|Default|GetRightTurnVelocity))
  (bind _returnvalue (+ _leftvelocity _leftturnvelocity))
  (bind _returnvalue_2 (+ _rightvelocity _rightturnvelocity))
  (Class|PhysicsConstraintComponent|SetAngularVelocityTarget (Variables|Default|GetPC_WheelFL) (Math|Vector|MakeVector 0.0 _returnvalue 0.0))
  (Class|PhysicsConstraintComponent|SetAngularVelocityTarget (Variables|Default|GetPC_WheelRL) (Math|Vector|MakeVector 0.0 _returnvalue 0.0))
  (Class|PhysicsConstraintComponent|SetAngularVelocityTarget (Variables|Default|GetPC_WheelFR) (Math|Vector|MakeVector 0.0 _returnvalue_2 0.0))
  (Class|PhysicsConstraintComponent|SetAngularVelocityTarget (Variables|Default|GetPC_WheelRR) (Math|Vector|MakeVector 0.0 _returnvalue_2 0.0)))

(fn WakeRigidBody
  (Class|PrimitiveComponent|WakeAllRigidBodies (Variables|Default|GetWheelFL))
  (Class|PrimitiveComponent|WakeAllRigidBodies (Variables|Default|GetWheelRL))
  (Class|PrimitiveComponent|WakeAllRigidBodies (Variables|Default|GetWheelFR))
  (Class|PrimitiveComponent|WakeAllRigidBodies (Variables|Default|GetWheelRR)))

(fn CompensatePitch
  (bind _body (Variables|Default|GetBody))
  (bind _returnvalue (Transformation|GetRelativeTransform _body))
  (Transformation|SetRelativeRotation _body (Math|Rotator|MakeRotator (.roll (.rotation _returnvalue)) 0.0 (.yaw (.rotation _returnvalue))) false false))